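; BP_KnightPrisoner is an interactable prisoner character that rewards XP to the player who interacts with it.
; It loops an idle animation on its skeletal mesh from BeginPlay.
; Interact casts the instigator's player state to US_PlayerState, adds EarnedXp, then switches the mesh to a looping cheer through CharacterCheer.
; CanInteract has no logic, and Interact itself does not guard against repeated rewards.
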(event `self.ReceiveBeginPlay`
  (`SkeletalMeshComponent.PlayAnimation` (`self.SkeletalMesh`) (`self.MontageIdle`) true))

(event `CharacterCheer`
  (`SkeletalMeshComponent.PlayAnimation` (`self.SkeletalMesh`) (`self.MontageCheer`) true))

(event `self.Interact`
  (params (CharacterInstigator :type "US_Character Object Reference"))
  (bind _asus_player_state (cast `US_PlayerState` (`Pawn.PlayerState` CharacterInstigator)))
  (`US_PlayerState.AddXp` _asus_player_state (`self.EarnedXp`))
  (`self.CharacterCheer`))

(fn `CanInteract`
  (params (CharacterInstigator :type "US_Character Object Reference")))

(fn `UserConstructionScript`)